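; Player controller that handles character input and runs an on-screen match timer.
; Input events move the player character along the controller's forward and right vectors, control look and jumping, and forward Fire to BP_Player.
; Tick accumulates time and prints it against TotalTime as debug text.
; At a hard-coded three-minute limit, independent of TotalTime, it prints a Korean time-up message and resets the timer after a short Delay.
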(event EventTick
  (params (DeltaSeconds :type Float%20%28single-precision%29))
  (bind _totaltime (Variables|Default|GetTotalTime))
  (Variables|Default|SetTimer (+ DeltaSeconds (Variables|Default|GetTimer)))
  (if (< (Variables|Default|GetTimer) 1.8e+02)
    (Development|PrintString (Utilities|String|ToString(Text) (Utilities|Text|FormatText "{0}분 {1}초 / {2}분 {3}초" (/ (Variables|Default|GetTimer) 60) (Math|Integer|%(Integer) (Math|Float|Truncate (Variables|Default|GetTimer)) 60) (/ _totaltime 60) (Math|Integer|%(Integer) _totaltime 60))) true true "(R=0.000000,G=0.660000,B=1.000000,A=1.000000)" 0.0)
    (else
      (Development|PrintString "시간이 종료되었습니다!")
      (Utilities|FlowControl|Delay 3.0)
      (Variables|Default|SetTimer 0.0))))

(event Input|ActionEvents|InputActionJump
  (params (Key :type Key%20Structure :default "None"))
  (bind _returnvalue (Game|GetPlayerCharacter 0))
  ;[0.15 0.15 0.15 0.5] 점프
  (:Pressed
    (Character|Jump _returnvalue))
  (:Released
    (Character|StopJumping _returnvalue)))

(event Input|ActionEvents|InputActionFire
  (params (Key :type Key%20Structure :default "None"))
  ;[0.15 0.15 0.15 0.5] 공격
  (:Pressed
    (bind _asbp_player (Utilities|Casting|CastToBP_Player (Game|GetPlayerCharacter 0)))
    (Default|Fire _asbp_player)))

(event Input|AxisEvents|InputAxisMoveForward
  (params (AxisValue :type Float%20%28single-precision%29))
  ;[0.15 0.15 0.15 0.5] W, S 이동
  (Pawn|Input|AddMovementInput (Game|GetPlayerCharacter 0) (Transformation|GetActorForwardVector) AxisValue false))

(event Input|AxisEvents|InputAxisMoveRight
  (params (AxisValue :type Float%20%28single-precision%29))
  ;[0.15 0.15 0.15 0.5] A, D 이동
  (Pawn|Input|AddMovementInput (Game|GetPlayerCharacter 0) (Transformation|GetActorRightVector) AxisValue false))

(event Input|AxisEvents|InputAxisTurn
  (params (AxisValue :type Float%20%28single-precision%29))
  ;[0.15 0.15 0.15 0.5] 가로축 회전
  (Class|PlayerController|AddYawInput AxisValue))

(event Input|AxisEvents|InputAxisLookUp
  (params (AxisValue :type Float%20%28single-precision%29))
  ;[0.15 0.15 0.15 0.5] 세로축 회전
  (Class|PlayerController|AddPitchInput AxisValue))

(fn ConstructionScript)