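; Behavior tree service that tells an AI pawn when the player is nearby through the Player blackboard key.
; On activation it waits briefly, then caches the BP_Player actor found with GetActorOfClass.
; Each tick, while that reference is valid, it sets the key to the player within a fixed straight-line distance of the controlled pawn and clears it otherwise, with no sight check.
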(event EventReceiveTickAI
  (params (OwnerController :type AI%20Controller%20Object%20Reference) (ControlledPawn :type Pawn%20Object%20Reference) (DeltaSeconds :type Float%20%28single-precision%29))
  (Utilities|IsValid (Variables|Default|GetBP_Player)
    (:Is%20Valid
      (if (< (Math|Vector|VectorLength (- (Transformation|GetActorLocation (Variables|Default|GetBP_Player)) (Transformation|GetActorLocation ControlledPawn))) 8e+02)
        (Class|BTFunctionLibrary|SetBlackboardValueasObject (Variables|Default|GetPlayer) (Variables|Default|GetBP_Player))
        (else
          (Class|BTFunctionLibrary|SetBlackboardValueasObject (Variables|Default|GetPlayer)))))))

(event EventReceiveActivationAI
  (params (OwnerController :type AI%20Controller%20Object%20Reference) (ControlledPawn :type Pawn%20Object%20Reference))
  (Utilities|FlowControl|Delay 0.2)
  (bind _returnvalue (Actor|GetActorOfClass "/Game/Blueprints/BP_Player.BP_Player_C"))
  (Variables|Default|SetBP_Player _returnvalue))