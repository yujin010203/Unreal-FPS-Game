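; Game mode Blueprint that populates the level with monsters and sets up a test UI.
; On BeginPlay it runs a ten-pass loop, each spawning BP_Monster at a random reachable navmesh point around the origin.
; The same loop body also creates a WBP_UITest widget every pass and picks UI-only or game-only input from IsPressed.
; A SpawnMonster event respawns one monster the same way and decrements SpawnCount.
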(event Custom|SpawnMonster
  ;[0.15 0.15 0.15 0.5] 몬스터 리스폰
  (Game|SpawnActorfromClass "/Game/Blueprints/BP_Monster.BP_Monster_C" (Math|Transform|MakeTransform (.RandomLocation (AI|Navigation|GetRandomReachablePointinRadius (Variables|Default|GetOriginVector) 3e+03 0 0)) "0, 0, 0" "1.000000,1.000000,1.000000") "Undefined" "MultiplyWithRoot" 0 0)
  (Variables|Default|SetSpawnCount (- (Variables|Default|GetSpawnCount) 1)))

(event EventBeginPlay
  (bind _returnvalue (Game|GetPlayerController 0))
  ;[0.15 0.15 0.15 0.5] 몬스터 랜덤 위치 생성
  (for _index (range 1 10)
    (Game|SpawnActorfromClass "/Game/Blueprints/BP_Monster.BP_Monster_C" (Math|Transform|MakeTransform (.RandomLocation (AI|Navigation|GetRandomReachablePointinRadius (Variables|Default|GetOriginVector) 3e+03 0 0)) "0, 0, 0" "1.000000,1.000000,1.000000") "Undefined" "MultiplyWithRoot" 0 0)
    (bind _returnvalue_2 (UserInterface|CreateWidget "/Game/UI/WBP_UITest.WBP_UITest_C"))
    (bind _output_get (Variables|Default|SetUITest _returnvalue_2))
    (UserInterface|Viewport|AddtoViewport _output_get 0)
    (if (Variables|Default|GetIsPressed)
      (Input|SetInputModeUIOnly _returnvalue 0 "DoNotLock" false)
      (Variables|/Script/Engine.PlayerController|SetbShowMouseCursor _returnvalue true)
      (else
        (Input|SetInputModeGameOnly (Game|GetPlayerController 0) false)))))

(event EventTick
  (params (DeltaSeconds :type Float%20%28single-precision%29)))

(fn ConstructionScript)