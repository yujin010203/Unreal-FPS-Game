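; BP_Player is the player character, with hit points, a hitscan Fire action and an upward-launch SuperJump.
; Fire plays a montage, traces from screen center and subtracts fixed damage from a hit BP_Monster's HP.
; A second trace from the arrow_anchor socket to that hit point only draws debug, as its result is unused.
; Tick prints HP and, at zero or below, flags death and quits the game.
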(event EventBeginPlay
  (Variables|Default|SetPlayerHP (Variables|Default|GetPlayerHP)))

(event Collision|EventActorBeginOverlap
  (params (OtherActor :type Actor%20Object%20Reference)))

(event EventTick
  (params (DeltaSeconds :type Float%20%28single-precision%29))
  (Development|PrintString (Utilities|String|ToString(Text) (Utilities|Text|FormatText "Player HP : {0}" (Variables|Default|GetPlayerHP))) true true "(R=0.000000,G=0.660000,B=1.000000,A=1.000000)" 0.0)
  (if (<= (Variables|Default|GetPlayerHP) 0)
    (Variables|Default|SetIsDead true)
    (Development|PrintString "게임이 종료되었습니다!")
    (Game|QuitGame 0 "Quit" false)))

(fn ConstructionScript)

(fn Fire
  (bind _returnvalue (Game|GetPlayerController 0))
  (bind _returnvalue_2 (Viewport|GetViewportSize))
  (bind _returnvalue_3 (/ (.y _returnvalue_2) 2.0))
  (bind _returnvalue_4 (/ (.x _returnvalue_2) 2.0))
  (bind (_worldposition _worlddirection) (Class|GameplayStatics|DeprojectScreentoWorld _returnvalue (Math|Vector2D|MakeVector2D _returnvalue_4 _returnvalue_3)))
  (Animation|PlayAnimMontage "/Game/Animations/AM_Fire.AM_Fire" 1.0 "None")
  (bind _outhit (Collision|LineTraceByChannel _worldposition (+ _worldposition (* _worlddirection 5e+03)) "TraceTypeQuery1" false 0 "ForDuration" true "(R=1.000000,G=0.000000,B=0.000000,A=1.000000)" "(R=0.000000,G=1.000000,B=0.000000,A=1.000000)" 0.0))
  (Collision|LineTraceByChannel (.location (Transformation|GetSocketTransform (Variables|Character|GetMesh) "arrow_anchor" "RTS_World")) (.Location (Collision|BreakHitResult _outhit)) "TraceTypeQuery1" false 0 "ForDuration" true "(R=1.000000,G=0.000000,B=0.000000,A=1.000000)" "(R=0.000000,G=1.000000,B=0.000000,A=1.000000)" 0.0)
  (bind _asbp_monster (Utilities|Casting|CastToBP_Monster (.HitActor (Collision|BreakHitResult _outhit))))
  (Variables|/Game/Blueprints/BP_Monster.BP_Monster_C|SetMonsterHP _asbp_monster (- (Variables|/Game/Blueprints/BP_Monster.BP_Monster_C|GetMonsterHP _asbp_monster) 3)))

(fn SuperJump
  (Character|LaunchCharacter "0.000000,0.000000,1000.000000" false false))